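; BP_Enemy is an enemy pawn that travels through a Destination array using AI movement and prints any damage it takes.
; BeginPlay starts MoveTo, which issues AIMoveTo to the point at Index while that index is valid.
; On success it waits briefly, calls MoveTo again and only then increments Index, with no wraparound or failure handling.
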(event Custom|MoveTo
  (if (Utilities|Array|IsValidIndex (Variables|Default|GetDestination) (Variables|Default|GetIndex))
    (AI|AIMoveTo self (Utilities|Array|Get(acopy) (Variables|Default|GetDestination) (Variables|Default|GetIndex)) 0 5.0 false
      (:OnSuccess
        (Utilities|FlowControl|Delay 0.2)
        (CallFunction|Moveto)
        (Math|Integer|IncrementInt (Variables|Default|GetIndex))))))

(event EventBeginPlay
  (CallFunction|Moveto))

(event Collision|EventActorBeginOverlap
  (params (OtherActor :type Actor%20Object%20Reference)))

(event EventTick
  (params (DeltaSeconds :type Float%20%28single-precision%29)))

(event Game|Damage|EventAnyDamage
  (params (Damage :type Float%20%28single-precision%29) (DamageType :type Damage%20Type%20Object%20Reference) (InstigatedBy :type Controller%20Object%20Reference) (DamageCauser :type Actor%20Object%20Reference))
  (Development|PrintString (Utilities|String|ToString(Float) Damage)))

(fn ConstructionScript)