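; BP_EnemyCube is an enemy cube actor that tracks its own health and can reduce the health shown in WBP_HealtBar.
; TakeDamage subtracts damage from CurrentHealth, then destroys the cube and prints a debug message at zero or below.
; A Timer event calls ReduceHealt on top-level health bar widgets and destroys the cube, but its SetTimerByFunctionName setup is unconnected, so this Blueprint never schedules it.
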(event Custom|Timer
  (bind _foundwidgets (Widget|GetAllWidgetsOfClass "/Game/Blueprints/WBP_HealtBar.WBP_HealtBar_C" true))
  (Default|ReduceHealt _foundwidgets)
  (Actor|DestroyActor))

(event EventBeginPlay)

(event Collision|EventActorBeginOverlap
  (params (OtherActor :type Actor%20Object%20Reference)))

(event EventTick
  (params (DeltaSeconds :type Float%20%28single-precision%29)))

(fn ConstructionScript)

(fn TakeDamage
  (params (DamageAmount :type Float%20%28double-precision%29))
  (Variables|Default|SetCurrentHealth (- (Variables|Default|GetCurrentHealth) DamageAmount))
  (if (<= (Variables|Default|GetCurrentHealth) 0.0)
    (Actor|DestroyActor)
    (Development|PrintString "damage done")))