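; BP_MAINTurret1 is a turret that yaws toward a target and fires pairs of BP_Projectile from two muzzle points.
; Detection sphere overlaps, filtered by actor tag "None", start and clear a fast looping timer that updates rotation.
; A Delay inside that timer throttles firing, with BulletSpeed acting as the shot interval rather than velocity.
; The construction script sets the detection radius and shows the sphere in game when Debugg is on.
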(event OnComponentBeginOverlap(detection)
  (params (OverlappedComponent :type Primitive%20Component%20Object%20Reference) (OtherActor :type Actor%20Object%20Reference) (OtherComp :type Primitive%20Component%20Object%20Reference) (OtherBodyIndex :type Integer) (bFromSweep :type Boolean) (SweepResult :type Hit%20Result%20Structure%20%28by%20ref%29))
  (if (Actor|ActorHasTag OtherActor "None")
    (CallFunction|LookingatTarget)))

(event OnComponentEndOverlap(detection)
  (params (OverlappedComponent :type Primitive%20Component%20Object%20Reference) (OtherActor :type Actor%20Object%20Reference) (OtherComp :type Primitive%20Component%20Object%20Reference) (OtherBodyIndex :type Integer))
  (if (Actor|ActorHasTag OtherActor "None")
    (Utilities|Time|ClearandInvalidateTimerbyHandle (Variables|Default|GetTimerLookAt))
    (Variables|Default|SetTimerLookAt "")))

(event Custom|LookingAtTarget
  (params (Actor :type Actor%20Object%20Reference))
  (bind _returnvalue (Utilities|Time|SetTimerbyEvent (delegate Custom|LookTimer) 0.01 true))
  (Variables|Default|SetTimerLookAt _returnvalue))

(event Custom|LookTimer
  (Transformation|SetActorRotation (Math|Rotator|MakeRotator 0.0 0.0 (.yaw (Math|Rotator|FindLookatRotation (Transformation|GetActorLocation) (Transformation|GetActorLocation (stale Custom|LookingAtTarget Actor))))))
  (Utilities|FlowControl|Delay (Variables|Default|GetBulletSpeed))
  (Game|SpawnActorfromClass "/Game/BP_Projectile.BP_Projectile_C" (Transformation|GetWorldTransform (Variables|Default|GetBullet)) "Undefined" "MultiplyWithRoot" 0 0)
  (Game|SpawnActorfromClass "/Game/BP_Projectile.BP_Projectile_C" (Transformation|GetWorldTransform (Variables|Default|GetBullet1)) "Undefined" "MultiplyWithRoot" 0 0))

(fn ConstructionScript
  (Development|SetHiddeninGame (Variables|Default|Getdetection) (select (Variables|Default|GetDebugg) false true) false)
  (Components|Sphere|SetSphereRadius (Variables|Default|Getdetection) (Variables|Default|GetIn%20Sphere%20Radius) true))