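; BP_Turret is a turret actor meant to target BP_Enemy actors on a looping FireRate timer.
; Each Shoot scans all enemies and stores one closer to its Arrow than ClosestDistance as TargetEnemy, then zeroes that threshold rather than storing the measured distance.
; Logic to aim the Scene and Arrow, spawn BP_Projectile and set its damage is present but disconnected, so it never fires.
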(event EventBeginPlay
  (Utilities|Time|SetTimerbyFunctionName 0 "Shoot" (Variables|Default|GetFireRate) true))

(fn ConstructionScript)

(fn Shoot
  (bind _outactors (Actor|GetAllActorsOfClass "/Game/ENEMY/BP_Enemy.BP_Enemy_C"))
  (for _array_element _outactors
    (if (< (Math|Vector|Distance(Vector) (Transformation|GetActorLocation _array_element) (Transformation|GetWorldLocation (Variables|Default|GetArrow))) (LocalVariables|GetClosestDistance))
      (LocalVariables|SetClosestDistance 0.0)
      (LocalVariables|SetTargetEnemy _array_element))))