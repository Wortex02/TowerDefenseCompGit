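; BP_Enemy is an enemy that, shortly after spawning, walks slowly toward a randomly chosen BP_goal actor.
; BeginPlay sets its walk speed and calls AIMoveTo, with a random index whose upper bound is the array length, so it can overrun.
; Both success and failure only cast the player pawn to BP_TowerPawn.
; The health subtraction and delayed self-destroy logic is disconnected and never runs.
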(event EventBeginPlay
  (Utilities|FlowControl|Delay 0.2)
  (Variables|/Script/Engine.CharacterMovementComponent|SetMaxWalkSpeed (Variables|Character|GetCharacterMovement) 5e+01)
  (bind _outactors (Actor|GetAllActorsOfClass "/Game/Enemy/BP_goal.BP_goal_C"))
  (AI|AIMoveTo self "0, 0, 0" (Utilities|Array|Get(acopy) _outactors (Math|Random|RandomIntegerinRange 0 (Utilities|Array|Length _outactors))) 5.0 false
    (:OnSuccess
      _)
    (:OnFail
      _))
  (bind _asbp_tower_pawn (Utilities|Casting|CastToBP_TowerPawn (Game|Player|GetPlayerPawn 0))))

(event Collision|EventActorBeginOverlap
  (params (OtherActor :type Actor%20Object%20Reference)))

(event EventTick
  (params (DeltaSeconds :type Float%20%28single-precision%29)))

(fn ConstructionScript
  (|CallParentFunction))