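; Test turret actor that turns to face the player and fires projectiles while the player is inside its detection sphere.
; Overlap begin starts a fast looping timer that interpolates yaw toward the player, and overlap end clears it.
; The same timer feeds a Delay, so BulletSpeed acts as the firing interval for projectile pairs spawned at two muzzle components.
; Construction script sets the sphere radius and debug visibility.
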(event OnComponentBeginOverlap(detection)
  (params (OverlappedComponent :type Primitive%20Component%20Object%20Reference) (OtherActor :type Actor%20Object%20Reference) (OtherComp :type Primitive%20Component%20Object%20Reference) (OtherBodyIndex :type Integer) (bFromSweep :type Boolean) (SweepResult :type Hit%20Result%20Structure%20%28by%20ref%29))
  (if (== OtherActor (Game|GetPlayerCharacter 0))
    (CallFunction|LookingatTarget)))

(event OnComponentEndOverlap(detection)
  (params (OverlappedComponent :type Primitive%20Component%20Object%20Reference) (OtherActor :type Actor%20Object%20Reference) (OtherComp :type Primitive%20Component%20Object%20Reference) (OtherBodyIndex :type Integer))
  (if (== OtherActor (Game|GetPlayerCharacter 0))
    (Utilities|Time|ClearandInvalidateTimerbyHandle (Variables|Default|GetTimerLookAt))
    (Variables|Default|SetTimerLookAt "")))

(event Custom|LookingAtTarget
  (bind _returnvalue (Utilities|Time|SetTimerbyEvent (delegate Custom|LookTimer) 0.01 true))
  (Variables|Default|SetTimerLookAt _returnvalue))

(event Custom|LookTimer
  (Transformation|SetActorRotation (Math|Rotator|MakeRotator 0.0 0.0 (.yaw (Math|Interpolation|RInterpTo (Transformation|GetActorRotation) (Math|Rotator|FindLookatRotation (Transformation|GetActorLocation) (Transformation|GetActorLocation (Game|GetPlayerCharacter 0))) (Utilities|Time|GetWorldDeltaSeconds) (* 1e+02 2.0)))))
  (Utilities|FlowControl|Delay (Variables|Default|GetBulletSpeed))
  (Game|SpawnActorfromClass "/Game/BP_Projectile.BP_Projectile_C" (Transformation|GetWorldTransform (Variables|Default|GetBullet)) "Undefined" "MultiplyWithRoot" 0 0)
  (Game|SpawnActorfromClass "/Game/BP_Projectile.BP_Projectile_C" (Transformation|GetWorldTransform (Variables|Default|GetBullet1)) "Undefined" "MultiplyWithRoot" 0 0))

(fn ConstructionScript
  (Development|SetHiddeninGame (Variables|Default|Getdetection) (select (Variables|Default|GetDebugg) false true) false)
  (Components|Sphere|SetSphereRadius (Variables|Default|Getdetection) (Variables|Default|GetIn%20Sphere%20Radius) true))